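; BP_SaveGameData holds the player's saved visual choices: character, hat and hat color IDs.
; SetSavedVisuals compares each incoming ID with the stored one and overwrites only those that differ.
; It returns a SomethingChanged flag so the caller knows when to update visuals.
; The function only sets variables and does not write the save to disk itself.
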(fn `SetSavedVisuals`
  (params (NewCharacterID :type Integer) (NewHatID :type Integer) (NewHatColorID :type Integer))
  (returns (bVisualsChanged :type Boolean))
  (locals (bSomethingChanged :type Boolean) (LocalCharacterID :type Integer) (LocalHatID :type Integer) (LocalHatColorID :type Integer))
  ;[1 1 1] Cache local variables
  (set `local.LocalCharacterID` NewCharacterID)
  (set `local.LocalHatID` NewHatID)
  (set `local.LocalHatColorID` NewHatColorID)
  ;[1 1 1] Save our new visual information and keep track whether something has changed
  (`|ExecutionSequence`
    (:`then_0`
      (if (!= (`local.LocalCharacterID`) (`self.CharacterID`))
        (set `self.CharacterID` (`local.LocalCharacterID`))
        (set `local.bSomethingChanged` true)))
    (:`then_1`
      (if (!= (`local.LocalHatID`) (`self.HatID`))
        (set `self.HatID` (`local.LocalHatID`))
        (set `local.bSomethingChanged` true)))
    (:`then_2`
      (if (!= (`local.LocalHatColorID`) (`self.HatColorID`))
        (set `self.HatColorID` (`local.LocalHatColorID`))
        (set `local.bSomethingChanged` true)))
    (:`then_3`
      ;[1 1 1] Return, letting the caller know something has changed so that it can appropriately update visuals
      (return (`local.bSomethingChanged`)))))